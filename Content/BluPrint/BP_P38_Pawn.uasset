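; BP_P38_Pawn is a player-controllable P-38 plane pawn that flies forward continuously.
; Every tick it spins the left and right propeller components at a fixed, frame-rate-independent speed and adds movement input along the actor's forward vector.
; Roll and Pitch axis inputs rotate the actor locally, scaled by delta time, so steering changes the direction of flight.
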(event `self.ReceiveTick`
  (params (DeltaSeconds :type "Float (single-precision)"))
  (`|ExecutionSequence`
    (:`then_0`
      ;[1 1 1] 오른쪽 프로펠러
      (`SceneComponent.K2_AddLocalRotation` (`self.Propeller Right`) (`KismetMathLibrary.MakeRotator` (* (`GameplayStatics.GetWorldDeltaSeconds`) 1080.0)) false false))
    (:`then_1`
      ;[1 1 1] 왼쪽 프로펠러
      (`SceneComponent.K2_AddLocalRotation` (`self.PropellerLeft`) (`KismetMathLibrary.MakeRotator` (* (`GameplayStatics.GetWorldDeltaSeconds`) 1080.0)) false false))
    (:`then_2`
      ;[1 1 1] P38이동
      (`self.AddMovementInput` (`self.GetActorForwardVector`)))))

(event `InputAxis|Roll`
  (params (AxisValue :type "Float (single-precision)"))
  (`self.K2_AddActorLocalRotation` (`KismetMathLibrary.MakeRotator` (* AxisValue 60.0 (`GameplayStatics.GetWorldDeltaSeconds`)))))

(event `InputAxis|Pitch`
  (params (AxisValue :type "Float (single-precision)"))
  (`self.K2_AddActorLocalRotation` (`KismetMathLibrary.MakeRotator` 0.0 (* AxisValue 60.0 (`GameplayStatics.GetWorldDeltaSeconds`)))))

(fn `UserConstructionScript`)