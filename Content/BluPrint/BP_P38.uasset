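; BP_P38 is a P-38 aircraft Blueprint that animates its two propellers.
; Each Tick, a Sequence adds local roll to the right and left propeller components at the same fixed rate, scaled by world delta seconds so the spin is frame-rate independent.
; It contains no movement logic, and its construction script is empty.
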(event `self.ReceiveTick`
  (params (DeltaSeconds :type "Float (single-precision)"))
  (`|ExecutionSequence`
    (:`then_0`
      ;[1 1 1] 오른쪽 프로펠러
      (`SceneComponent.K2_AddLocalRotation` (`self.Propeller Right`) (`KismetMathLibrary.MakeRotator` (* (`GameplayStatics.GetWorldDeltaSeconds`) 1080.0)) false false))
    (:`then_1`
      ;[1 1 1] 왼쪽 프로펠러
      (`SceneComponent.K2_AddLocalRotation` (`self.PropellerLeft`) (`KismetMathLibrary.MakeRotator` (* (`GameplayStatics.GetWorldDeltaSeconds`) 1080.0)) false false))))

(fn `UserConstructionScript`)