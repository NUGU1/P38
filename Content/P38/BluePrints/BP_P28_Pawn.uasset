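; Player-controlled propeller plane pawn that flies constantly forward and fires rockets.
; Roll and Pitch axis inputs rotate the actor locally, scaled by RotateSpeed and delta time.
; Tick spins both propeller components and adds forward movement input scaled by Boost, which the Boost action raises while held and lowers on release.
; The Fire action spawns a BP_Rocket at the Arrow component's world transform.
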(event `InputAxis|Roll`
  (params (AxisValue :type "Float (single-precision)"))
  (`self.K2_AddActorLocalRotation` (`KismetMathLibrary.MakeRotator` (* AxisValue (`self.Rotate Speed`) (`GameplayStatics.GetWorldDeltaSeconds`)))))

(event `self.ReceiveTick`
  (params (DeltaSeconds :type "Float (single-precision)"))
  (`|ExecutionSequence`
    (:`then_0`
      ;[1 1 1] Left Propeller Rotation
      (`SceneComponent.K2_AddLocalRotation` (`self.Propeller Left`) (`KismetMathLibrary.MakeRotator` (* (`GameplayStatics.GetWorldDeltaSeconds`) (`self.Propeller Rotate Speed`))) false false))
    (:`then_1`
      ;[1 1 1] Right Propeller Rotation
      (`SceneComponent.K2_AddLocalRotation` (`self.Propeller Right`) (`KismetMathLibrary.MakeRotator` (* (`GameplayStatics.GetWorldDeltaSeconds`) (`self.Propeller Rotate Speed`))) false false))
    (:`then_2`
      (`self.AddMovementInput` (`self.GetActorForwardVector`) (`self.Boost`)))))

(event `InputAxis|Pitch`
  (params (AxisValue :type "Float (single-precision)"))
  (`self.K2_AddActorLocalRotation` (`KismetMathLibrary.MakeRotator` 0.0 (* AxisValue (`self.Rotate Speed`) (`GameplayStatics.GetWorldDeltaSeconds`)))))

(event `InputAction|Fire`
  (params (Key :type "Key Structure"))
  (:`Pressed`
    (`|SpawnActorFromClass` "/Game/P38/BluePrints/BP_Rocket.BP_Rocket_C" (`SceneComponent.K2_GetComponentToWorld` (`self.Arrow`)) "Undefined" "OverrideRootScale" null null)))

(event `InputAction|Boost`
  (params (Key :type "Key Structure"))
  (:`Pressed`
    (set `self.Boost` 1.0))
  (:`Released`
    (set `self.Boost` 0.2)))

(fn `UserConstructionScript`)